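; Player controller for a networked chess game that handles board clicks, text chat and pausing.
; Left clicks send the cursor hit location to the first BP_ChessBoard via ClickReplicationClient; a ClickReplicationServer branch is left unconnected.
; Chat messages, tagged with the player's name, fan out through BP_GameMode's controller list to each chat window.
; M opens the chat widget and P opens the pause menu and pauses the game, creating each widget on demand.
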(event Custom|GetChatMessage
  (params (TextToSend :type Text))
  ;[1 1 1] Обработка сообщений чата
  (Variables|Default|SetSenderText TextToSend)
  (Variables|Default|SetSenderName (.MyPlayerName (Utilities|Struct|BreakPlayerInfo (Variables|Default|GetPlayerSetting))))
  (bind _asbp_game_mode (Utilities|Casting|CastToBP_GameMode (Game|GetGameMode)))
  (for _array_element (Variables|/Game/BP_GameMode.BP_GameMode_C|GetAllPlayerControllers _asbp_game_mode)
    (CallFunction|UpdateChat _array_element (Variables|Default|GetSenderName) (Variables|Default|GetSenderText))))

(event Custom|UpdateChat
  (params (Sender :type Text) (Text :type Text))
  ;[1 1 1] Вывод сообщения в окно чата
  (Default|UpdateChatWindow (Variables|/Game/UI/AllLevels/PlayChat.PlayChat_C|GetChatWindow (Variables|Default|GetChatWindowWB)) Sender Text))

(event EventBeginPlay
  ;[1 1 1] Установка курсора
  (Variables|Default|SetbShowMouseCursor true)
  (bind _outactors (Actor|GetAllActorsOfClass "/Game/Player/BP_ChessBoard.BP_ChessBoard_C"))
  (Variables|Default|SetChessBoard_Click (Utilities|Array|Get(acopy) _outactors)))

(event Input|MouseEvents|LeftMouseButton
  (params (Key :type Key%20Structure :default "None"))
  (:Pressed
    (Default|ClickReplicationClient (Variables|Default|GetChessBoard_Click) (.Location (Collision|BreakHitResult (.HitResult (Game|Player|GetHitResultUnderCursorbyChannel "TraceTypeQuery1" true)))))))

(event Input|KeyboardEvents|M
  (params (Key :type Key%20Structure :default "None"))
  ;[1 1 1] Включение чата
  (:Pressed
    (Utilities|IsValid (Variables|Default|GetChatWindowWB)
      (:Is%20Valid
        _)
      (:Is%20Not%20Valid
        (bind _returnvalue (UserInterface|CreateWidget "/Game/UI/AllLevels/PlayChat.PlayChat_C"))
        (Variables|Default|SetChatWindowWB _returnvalue)))
    (UserInterface|Viewport|AddtoViewport (Variables|Default|GetChatWindowWB) 0)))

(event Input|KeyboardEvents|P
  (params (Key :type Key%20Structure :default "None"))
  ;[1 1 1] Пауза
  (:Pressed
    (Utilities|IsValid (Variables|Default|GetPauseWB)
      (:Is%20Valid
        _)
      (:Is%20Not%20Valid
        (bind _returnvalue (UserInterface|CreateWidget "/Game/UI/AllLevels/Pause.Pause_C"))
        (Variables|Default|SetPauseWB _returnvalue)))
    (UserInterface|Viewport|AddtoViewport (Variables|Default|GetPauseWB) 0)
    (Game|SetGamePaused true)))

(fn ConstructionScript)